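; BP_FlashlightMaster is a flashlight item Blueprint, named as a master class, that turns a Beam component on and off.
; SetupItem applies the IsActive state to the Beam's visibility, and ToggleLight flips both IsActive and that visibility.
; BeginPlay, overlap and Tick are disabled stubs, and the construction script only calls its parent.
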(event Custom|ToggleLight
  (bind _beam (Variables|Default|GetBeam))
  (if (Variables|Default|GetisActive)
    (Rendering|SetVisibility _beam false false)
    (Variables|Default|SetisActive false)
    (else
      (Rendering|SetVisibility _beam true false)
      (Variables|Default|SetisActive true))))

(event EventBeginPlay
  (|CallParentFunction) ; This node is disabled and will not be called.\nDrag off pins to build functionality.
)

(event Collision|EventActorBeginOverlap
  (params (OtherActor :type Actor%20Object%20Reference))
  (|CallParentFunction OtherActor) ; This node is disabled and will not be called.\nDrag off pins to build functionality.
)

(event EventTick
  (params (DeltaSeconds :type Float%20%28single-precision%29))
  (|CallParentFunction DeltaSeconds) ; This node is disabled and will not be called.\nDrag off pins to build functionality.
)

(event EventSetupItem
  (Rendering|SetVisibility (Variables|Default|GetBeam) (Variables|Default|GetisActive) false))

(fn ConstructionScript
  (|CallParentFunction))