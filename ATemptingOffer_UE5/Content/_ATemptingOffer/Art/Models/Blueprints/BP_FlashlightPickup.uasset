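; BP_FlashlightPickup is a flashlight pickup item whose beam can be switched on and off.
; On BeginPlay and on SetupItem, it sets the Beam component's visibility to match the IsActive flag.
; SecondaryInteract toggles the beam's visibility and updates IsActive to the new state.
; The construction script only calls its parent.
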(event EventSetupItem
  (Rendering|SetVisibility (Variables|Default|GetBeam) (Variables|Default|GetisActive) false))

(event EventBeginPlay
  (Rendering|SetVisibility (Variables|Default|GetBeam) (Variables|Default|GetisActive) false))

(event EventSecondaryInteract
  (params (InteractingPlayer :type BP%20Main%20Character%20Object%20Reference))
  (bind _beam (Variables|Default|GetBeam))
  (if (Variables|Default|GetisActive)
    (Rendering|SetVisibility _beam false false)
    (Variables|Default|SetisActive false)
    (else
      (Rendering|SetVisibility _beam true false)
      (Variables|Default|SetisActive true))))

(fn ConstructionScript
  (|CallParentFunction))