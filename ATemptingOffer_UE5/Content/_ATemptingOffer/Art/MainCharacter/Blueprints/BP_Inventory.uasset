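; BP_Inventory holds the main character's items in an Inventory array with a MaxSize capacity.
; Separate functions add an item, remove an item, and report whether the item count is still below MaxSize.
; The add function does not check capacity itself, so the limit depends on callers using CanAddItem.
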(fn AddItemtoInvemtory
  (params (Current%20Item :type BP%20Item%20Master%20Class%20Reference%20%28by%20ref%29))
  (Utilities|Array|Add (Variables|Default|GetInventory) Current%20Item))

(fn RemoveItemfromInventory
  (params (Current%20Item :type BP%20Item%20Master%20Class%20Reference%20%28by%20ref%29))
  (Utilities|Array|RemoveItem (Variables|Default|GetInventory) Current%20Item))

(fn CanAddItem
  (return (< (Utilities|Array|Length (Variables|Default|GetInventory)) (Variables|Default|GetMax%20Size))))