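; BP_InventoryTest is a simple inventory that tracks items in an array limited by MaxSize.
; BeginPlay pre-fills the array with empty slots, looping from zero through MaxSize inclusive.
; Adding writes the item into the first empty slot, while removing deletes the entry outright rather than clearing its slot.
; CanAddItem counts non-empty slots against MaxSize and resets the counter; a simpler length check is left unconnected.
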(event EventBeginPlay
  (for _index (range 0 (Variables|Default|GetMax%20Size))
    (Utilities|Array|Add (Variables|Default|GetInventory) 0)))

(fn AddItemtoInvemtory
  (params (Current%20Item :type BP%20Default%20Item%20Class%20Reference%20%28by%20ref%29))
  (bind _inventory (Variables|Default|GetInventory))
  (Utilities|Array|SetArrayElem _inventory (Utilities|Array|FindItem _inventory 0) Current%20Item))

(fn RemoveItemfromInventory
  (params (Current%20Item :type BP%20Default%20Item%20Class%20Reference%20%28by%20ref%29))
  (Utilities|Array|RemoveItem (Variables|Default|GetInventory) Current%20Item))

(fn CanAddItem
  (for _array_element (Variables|Default|GetInventory)
    (if (!= _array_element 0)
      (Math|Integer|IncrementInt (Variables|Default|GetCount))))
  (if (< (Variables|Default|GetCount) (Variables|Default|GetMax%20Size))
    (Variables|Default|SetCount 0)
    (return true)
    (else
      (Variables|Default|SetCount 0)
      (return false))))